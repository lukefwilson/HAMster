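; BP_BuildingBlock is a modular building piece made of four walls, a ceiling and a floor.
; Its construction script passes each part's Has flag, component and material variable to ToggleComponent.
; That function sets the material on element 0 of enabled parts and destroys disabled components rather than hiding them.
; The event graph holds only disabled stub events, so the Blueprint adds no runtime logic.
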(event EventBeginPlay)

(event Collision|EventActorBeginOverlap
  (params (OtherActor :type Actor%20Object%20Reference)))

(event EventTick
  (params (DeltaSeconds :type Float%20%28single-precision%29)))

(fn ConstructionScript
  (Utilities|FlowControl|Sequence
    (:then_0
      (CallFunction|ToggleComponent (Variables|Building|GetHasWall1) (Variables|Default|GetWall1) (Variables|Materials|GetWall1Material)))
    (:then_1
      (CallFunction|ToggleComponent (Variables|Building|GetHasWall2) (Variables|Default|GetWall2) (Variables|Materials|GetWall2Material)))
    (:then_2
      (CallFunction|ToggleComponent (Variables|Building|GetHasWall3) (Variables|Default|GetWall3) (Variables|Materials|GetWall3Material)))
    (:then_3
      (CallFunction|ToggleComponent (Variables|Building|GetHasWall4) (Variables|Default|GetWall4) (Variables|Materials|GetWall4Material)))
    (:then_4
      (CallFunction|ToggleComponent (Variables|Building|GetHasCeiling) (Variables|Default|GetCeiling) (Variables|Materials|GetCeilingMaterial)))
    (:then_5
      (CallFunction|ToggleComponent (Variables|Building|GetHasFloor) (Variables|Default|GetFloor) (Variables|Materials|GetFloorMaterial)))))

(fn ToggleComponent
  (params (Visible :type Boolean) (Component :type Static%20Mesh%20Component%20Object%20Reference) (Material :type Material%20Object%20Reference))
  (if Visible
    (Rendering|Material|SetMaterial Component 0 Material)
    (else
      (Components|DestroyComponent Component))))